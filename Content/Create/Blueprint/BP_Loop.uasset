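; BP_Loop is a procedural placement actor that arranges copies of the Sm_fish_NN static mesh along a horizontal circle or arc.
; Its construction script loops up to LastIndex, adding a mesh component at each step using degree-based sine and cosine at a fixed radius.
; The Value variable sets the total angle, divided evenly by LastIndex.
; The event graph holds only disabled placeholder events, so there is no runtime logic.
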(event EventBeginPlay)

(event Collision|EventActorBeginOverlap
  (params (OtherActor :type Actor%20Object%20Reference)))

(event EventTick
  (params (DeltaSeconds :type Float%20%28single-precision%29)))

(fn ConstructionScript
  (bind _last_index (Variables|Default|GetLast%20Index))
  (for _index (range 1 _last_index)
    (bind _returnvalue (AddComponent|AddStaticMeshComponent false (Math|Transform|MakeTransform (Math|Vector|MakeVector (* (Math|Trig|Sin(Degrees) (* (Math|Conversions|ToFloat(Integer) _index) (/ (Variables|Default|GetValue) _last_index))) 2e+02) (* (Math|Trig|Cos(Degrees) (* (Math|Conversions|ToFloat(Integer) _index) (/ (Variables|Default|GetValue) _last_index))) 2e+02) 0.0) "0, 0, 0" "1.000000,1.000000,1.000000")))
    (Components|StaticMesh|SetStaticMesh _returnvalue "/Game/Create/Mesh/Sm_fish_NN.Sm_fish_NN")))